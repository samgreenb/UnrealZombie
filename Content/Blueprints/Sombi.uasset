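; Zombie enemy pawn that chases the player and damages them on contact.
; On BeginPlay it issues a single AI MoveTo toward the player; overlap events track contact, and Tick applies damage on a timed cooldown while overlapping.
; ChangeLife subtracts health and, on death, notifies its Spawner, increments the score on the GameHUD widget found by class lookup, and destroys the actor.
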(event Collision|EventActorBeginOverlap
  (params (OtherActor :type Actor%20Object%20Reference))
  (bind _asplayer (Utilities|Casting|CastToPlayer OtherActor))
  (Variables|Default|Setplayer _asplayer)
  (Variables|Default|SetPlayerOverlap true))

(event Collision|EventActorEndOverlap
  (params (OtherActor :type Actor%20Object%20Reference))
  (Utilities|Casting|CastToPlayer OtherActor)
  (Variables|Default|SetPlayerOverlap false))

(event EventTick
  (params (DeltaSeconds :type Float%20%28single-precision%29))
  (Variables|Default|SetattackTimer (+ DeltaSeconds (Variables|Default|GetattackTimer)))
  (if (and (Variables|Default|GetPlayerOverlap) (> (Variables|Default|GetattackTimer) 2.0))
    (Variables|Default|SetattackTimer 0.0)
    (Default|ChangeLife (Variables|Default|Getplayer) 34)))

(event EventBeginPlay
  ;[1 1 1] Zombie Movement
  (AI|AIMoveTo self "0, 0, 0" (Game|GetPlayerCharacter 0) 5.0 false))

(fn ConstructionScript)

(fn ChangeLife
  (params (ChangeLife :type Integer))
  (bind _output_get (Variables|Default|SetLife (- (Variables|Default|GetLife) ChangeLife)))
  (Math|Integer|CompareInt _output_get 1
    (:<
      (Default|RemoveZombie (Variables|Default|GetSpawner))
      (bind _foundwidgets (Widget|GetAllWidgetsOfClass "/Game/Blueprints/GameHUD.GameHUD_C" true))
      (Variables|/Game/Blueprints/GameHUD.GameHUD_C|Setscore (Utilities|Array|Get(acopy) _foundwidgets) (+ (Variables|/Game/Blueprints/GameHUD.GameHUD_C|Getscore (Utilities|Array|Get(acopy) _foundwidgets)) 1))
      (Actor|DestroyActor))))