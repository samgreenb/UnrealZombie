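; ZombieSpawn is a spawner actor that keeps a small population of Sombi zombies at its location.
; A looping timer started on BeginPlay spawns a Sombi at the actor's position whenever its live count is below two, then increments the count.
; Each spawned zombie receives a reference back to the spawner, and RemoveZombie decrements the count so a replacement can spawn.
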(event Custom|ZombieSpawn
  (Math|Integer|CompareInt (Variables|Default|GetNumberZombies) 2
    (:<
      (bind _returnvalue (Game|SpawnActorfromClass "/Game/Blueprints/Sombi.Sombi_C" (Math|Transform|MakeTransform (Transformation|GetActorLocation) "0, 0, 0" "1.000000,1.000000,1.000000") "Undefined" "MultiplyWithRoot" 0 0))
      (Variables|/Game/Blueprints/Sombi.Sombi_C|SetSpawner _returnvalue self)
      (Variables|Default|SetNumberZombies (+ (Variables|Default|GetNumberZombies) 1)))))

(event EventBeginPlay
  (Utilities|Time|SetTimerbyEvent (delegate Custom|ZombieSpawn) 2.5 true))

(fn ConstructionScript)

(fn RemoveZombie
  (Variables|Default|SetNumberZombies (+ (Variables|Default|GetNumberZombies) -1)))